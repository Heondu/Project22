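; Ragdoll fighter character that trades punches with others of its class, running a physics-simulated mesh on a fight physics asset.
; Left clicks alternate left and right punch montages, briefly pausing simulation and enabling that hand's overlap collision.
; Hand overlaps subtract HP from other ragdoll characters.
; Tick updates the HP widget's progress bar and switches to the Ragdoll physics asset when HP reaches zero.
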(event OnComponentBeginOverlap(RightHand)
  (params (OverlappedComponent :type Primitive%20Component%20Object%20Reference) (OtherActor :type Actor%20Object%20Reference) (OtherComp :type Primitive%20Component%20Object%20Reference) (OtherBodyIndex :type Integer) (bFromSweep :type Boolean) (SweepResult :type Hit%20Result%20Structure%20%28by%20ref%29))
  (if (!= OtherActor self)
    (bind _asbp_ragdoll_character (Utilities|Casting|CastToBP_RagdollCharacter OtherActor))
    (Variables|BP_RagdollCharacter_C|SetHP _asbp_ragdoll_character (- (Variables|BP_RagdollCharacter_C|GetHP _asbp_ragdoll_character) 1.0))))

(event OnComponentBeginOverlap(LeftHand)
  (params (OverlappedComponent :type Primitive%20Component%20Object%20Reference) (OtherActor :type Actor%20Object%20Reference) (OtherComp :type Primitive%20Component%20Object%20Reference) (OtherBodyIndex :type Integer) (bFromSweep :type Boolean) (SweepResult :type Hit%20Result%20Structure%20%28by%20ref%29))
  (if (!= OtherActor self)
    (bind _asbp_ragdoll_character (Utilities|Casting|CastToBP_RagdollCharacter OtherActor))
    (Variables|BP_RagdollCharacter_C|SetHP _asbp_ragdoll_character (- (Variables|BP_RagdollCharacter_C|GetHP _asbp_ragdoll_character) 1.0))))

(event EventBeginPlay
  (bind _mesh (Variables|Character|GetMesh))
  (Components|SkinnedMesh|SetPhysicsAsset _mesh "/Game/Mannequin/Character/Mesh/FightPhysics.FightPhysics" false)
  (Physics|SetSimulatePhysics _mesh true))

(event EventTick
  (params (DeltaSeconds :type Float%20%28single-precision%29))
  (Utilities|FlowControl|Sequence
    (:then_0
      (if (== (Variables|Default|GetHP) 0.0)
        (Components|SkinnedMesh|SetPhysicsAsset (Variables|Character|GetMesh) "/Game/Mannequin/Character/Mesh/Ragdoll.Ragdoll" false)))
    (:then_1
      (bind _aswbp_hp (Utilities|Casting|CastToWBP_HP (UserInterface|GetUserWidgetObject (Variables|Default|GetHPWidget))))
      (Progress|SetPercent (Variables|/Game/MyContent/UI/WBP_HP.WBP_HP_C|GetProgressBar_0 _aswbp_hp) (/ (Variables|Default|GetHP) 1e+01)))))

(event Input|MouseEvents|LeftMouseButton
  (params (Key :type Key%20Structure :default "None"))
  (bind _mesh (Variables|Character|GetMesh))
  (bind _mesh_2 (Variables|Character|GetMesh))
  (bind _returnvalue (Components|SkeletalMesh|GetAnimInstance _mesh))
  (:Pressed
    (Utilities|FlowControl|FlipFlop
      (:A
        (Physics|SetSimulatePhysics _mesh false)
        (Animation|Montage|MontagePlay _returnvalue "/Game/MyContent/Animations/AM_LeftPunch_Mannequin.AM_LeftPunch_Mannequin" 2.0 "MontageLength" 0.0 true)
        (Collision|SetCollisionEnabled (Variables|Default|GetLeft%20Hand) "QueryOnly")
        (Utilities|FlowControl|Delay 0.5)
        (Physics|SetSimulatePhysics _mesh_2 true)
        (Collision|SetCollisionEnabled (Variables|Default|GetLeft%20Hand) "NoCollision"))
      (:B
        (Physics|SetSimulatePhysics _mesh false)
        (Animation|Montage|MontagePlay _returnvalue "/Game/MyContent/Animations/AM_RightPunch_Mannequin.AM_RightPunch_Mannequin" 2.0 "MontageLength" 0.0 true)
        (Collision|SetCollisionEnabled (Variables|Default|GetRight%20Hand) "QueryOnly")
        (Utilities|FlowControl|Delay 0.5)
        (Physics|SetSimulatePhysics _mesh_2 true)
        (Collision|SetCollisionEnabled (Variables|Default|GetRight%20Hand) "NoCollision")))))

(fn ConstructionScript)